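; Player controller for a Taiko drum game that handles startup and turns drum input into events.
; On BeginPlay it views through the first CameraActor found, shows WBP_StartMenu linked to the level's BP_GameFlow, and adds the IMC_Taiko mapping context.
; Enhanced Input actions fire the OnDon and OnKa dispatchers with an enum for the drum zone struck.
; Escape fires OnEsc, and a debug key only prints a message.
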(event `self.ReceiveBeginPlay`
  (`self.SetCamera`)
  (`self.SetUI`)
  (`self.SetInput`))

(event `EnhancedInput|/Game/Input/IA_DonL`
  (params (ActionValue :type Boolean) (ElapsedSeconds :type "Float (double-precision)") (TriggeredSeconds :type "Float (double-precision)") (InputAction :type "InputAction Object Reference" :default "/Game/Input/IA_DonL.IA_DonL"))
  (:`Triggered`
    (`self.OnDon` "NewEnumerator0")))

(event `EnhancedInput|/Game/Input/IA_DonR`
  (params (ActionValue :type Boolean) (ElapsedSeconds :type "Float (double-precision)") (TriggeredSeconds :type "Float (double-precision)") (InputAction :type "InputAction Object Reference" :default "/Game/Input/IA_DonR.IA_DonR"))
  (:`Triggered`
    (`self.OnDon` "NewEnumerator1")))

(event `EnhancedInput|/Game/Input/IA_KaL`
  (params (ActionValue :type Boolean) (ElapsedSeconds :type "Float (double-precision)") (TriggeredSeconds :type "Float (double-precision)") (InputAction :type "InputAction Object Reference" :default "/Game/Input/IA_KaL.IA_KaL"))
  (:`Triggered`
    (`self.OnKa` "NewEnumerator2")))

(event `EnhancedInput|/Game/Input/IA_KaR`
  (params (ActionValue :type Boolean) (ElapsedSeconds :type "Float (double-precision)") (TriggeredSeconds :type "Float (double-precision)") (InputAction :type "InputAction Object Reference" :default "/Game/Input/IA_KaR.IA_KaR"))
  (:`Triggered`
    (`self.OnKa` "NewEnumerator3")))

(event `EnhancedInput|/Game/Input/IA_Esc`
  (params (ActionValue :type Boolean) (ElapsedSeconds :type "Float (double-precision)") (TriggeredSeconds :type "Float (double-precision)") (InputAction :type "InputAction Object Reference" :default "/Game/Input/IA_Esc.IA_Esc"))
  (:`Triggered`
    (`self.OnEsc`)))

(event `EnhancedInput|/Game/Input/IA_DebugKey`
  (params (ActionValue :type Boolean) (ElapsedSeconds :type "Float (double-precision)") (TriggeredSeconds :type "Float (double-precision)") (InputAction :type "InputAction Object Reference" :default "/Game/Input/IA_DebugKey.IA_DebugKey"))
  (:`Triggered`
    (`KismetSystemLibrary.PrintString` "DEBUG_KEY")))

(fn `SetCamera`
  (bind _outactors (`GameplayStatics.GetAllActorsOfClass` "/Script/Engine.CameraActor"))
  (`self.SetViewTargetWithBlend` (`|GetArrayItem` _outactors)))

(fn `SetInput`
  (`EnhancedInputSubsystemInterface.AddMappingContext` (subsystem `EnhancedInputLocalPlayerSubsystem`) "/Game/Input/IMC_Taiko.IMC_Taiko" 0 (struct)))

(fn `SetUI`
  (bind _returnvalue (`GameplayStatics.GetActorOfClass` "/Game/BP/BP_GameFlow.BP_GameFlow_C"))
  (bind _returnvalue_2 (`|CreateWidget` "/Game/BP/WBP_StartMenu.WBP_StartMenu_C"))
  (set `/Game/BP/WBP_StartMenu.GameFlow` _returnvalue _returnvalue_2)
  (`UserWidget.AddToViewport` _returnvalue_2 0))

(fn `UserConstructionScript`)