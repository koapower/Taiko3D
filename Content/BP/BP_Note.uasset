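; BP_Note is a rhythm-game note that travels from a start point to a target, timed to reach it at its hit time.
; Setup initializes and shows it, picking a blue or red material by note type; Reset hides it and stops ticking, allowing reuse.
; While active and the map runs, Tick derives its position from the MusicManager's clock with a clamped lerp, keeping movement synced to the music.
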(event `self.ReceiveBeginPlay`)

(event `OnHit`)

(event `self.ReceiveTick`
  (params (DeltaSeconds :type "Float (single-precision)"))
  (if (and (and (`KismetSystemLibrary.IsValid` (`self.MusicManager`)) (`self.bActive`)) (`/Game/BP/BP_GameFlow.isMapRunning` (`self.GameFlow`)))
    (`self.UpdatePosition`)))

(fn `ChangeMaterial`
  (bind _cylinder (`self.Cylinder`))
  (if (== (`self.NoteType`) 8)
    ; BLUE
    (`PrimitiveComponent.CreateDynamicMaterialInstance` _cylinder 0 "/Game/Material/M_BlueNote_Inst.M_BlueNote_Inst" "None")
    (else
      ; RED
      (`PrimitiveComponent.CreateDynamicMaterialInstance` _cylinder 0 "/Game/Material/M_RedNote_Inst.M_RedNote_Inst" "None"))))

(fn `Reset`
  (`self.SetActorHiddenInGame` true)
  (`self.SetActorTickEnabled` false)
  (set `self.bActive` false))

(fn `Setup`
  (params (HitTime_ms :type Integer) (StartPos :type "Vector Structure") (EndPos :type "Vector Structure") (MusicManager :type "/Game/BP/BP_MusicManager Object Reference") (GameFlow :type "/Game/BP/BP_GameFlow Object Reference") (TravelTime :type "Float (double-precision)") (NoteType :type Integer))
  (set `self.HitTime_ms` HitTime_ms)
  (bind _output_get (set `self.StartLocation` StartPos))
  (set `self.TargetLocation` EndPos)
  (set `self.MusicManager` MusicManager)
  (set `self.GameFlow` GameFlow)
  (set `self.TravelTime_s` TravelTime)
  (set `self.NoteType` NoteType)
  (`self.ChangeMaterial`)
  (`self.K2_SetActorLocation` _output_get)
  (`self.SetActorHiddenInGame` false)
  (`self.SetActorTickEnabled` true)
  (set `self.bActive` true))

(fn `UpdatePosition`
  (bind _currenttime (`/Game/BP/BP_MusicManager.GetCurrentTime` (`self.MusicManager`)))
  (`self.K2_SetActorLocation` (`KismetMathLibrary.VLerp` (`self.TargetLocation`) (`self.StartLocation`) (`KismetMathLibrary.FClamp` (`KismetMathLibrary.SafeDivide` (- (`self.HitTime_ms`) (* _currenttime 1000.0)) (* (`self.TravelTime_s`) 1000.0))))))

(fn `UserConstructionScript`)