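; BP_GameFlow runs a map in a Taiko-style rhythm game: note spawning, music start, pause and restart.
; It loads beatmap rows from the Testmap DataTable, then each Tick spawns pooled notes TravelTime ahead of hit time, timed by MusicManager.
; Osu coordinates become directions on a ring of SpawnDistance, from which notes travel to the drum center.
; HitJudgementManager holds queued notes, clears misses and reports hits, returning notes to the pool.
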(event `OnNoteHit`
  (params (Note :type "/Game/BP/BP_Note Object Reference") (Result :type "/Game/BP/NoteHitResult Enum" :default "NewEnumerator0"))
  (`self.SolveOnNoteHit` Note)
  (`KismetSystemLibrary.PrintString` (`KismetStringLibrary.Concat_StrStr` (`KismetStringLibrary.Concat_StrStr` (`KismetSystemLibrary.GetDisplayName` Note) " OnNoteHit: ") (`|GetEnumeratorNameAsString` Result))))

(event `OnEsc`
  (`self.PauseMap`))

(event `self.ReceiveBeginPlay`
  (`self.InitNoteArray`)
  (add `/Game/BP/BP_HitJudgementManager.OnNoteHit` (`self.HitJudgementManager`) (delegate `OnNoteHit`))
  (bind _asbp_taiko_player_controller (cast `/Game/BP_TaikoPlayerController` (`GameplayStatics.GetPlayerController` 0)))
  (add `/Game/BP_TaikoPlayerController.OnEsc` _asbp_taiko_player_controller (delegate `OnEsc`)))

(event `self.ReceiveTick`
  (params (DeltaSeconds :type "Float (single-precision)"))
  (`self.CheckNoteSpawn`)
  (`/Game/BP/BP_HitJudgementManager.ClearMissedNotes` (`self.HitJudgementManager`)))

(fn `CheckNoteSpawn`
  (bind _currentnoteindex (`self.CurrentNoteIndex`))
  (bind _beatmaparray (`self.BeatmapArray`))
  (bind _returnvalue (`KismetArrayLibrary.Array_Length` _beatmaparray))
  (bind (_returnvalue_x _returnvalue_y _returnvalue_z) (`KismetMathLibrary.BreakVector` (`self.K2_GetActorLocation` (`self.DrumCenter`))))
  (bind _returnvalue_2 (+ _returnvalue_z 30.0))
  (if (< _currentnoteindex _returnvalue)
    (for _index (range _currentnoteindex _returnvalue)
      (bind _currenttime (`/Game/BP/BP_MusicManager.GetCurrentTime` (`self.MusicManager`)))
      (bind (_osux _osuy _hittime _param1 _hitsound) (break `/Game/BP/STR_NoteInfo` (`|GetArrayItem` _beatmaparray _index)))
      (if (>= (* (+ _currenttime (`self.TravelTime`)) 1000.0) _hittime)
        (bind _note (`/Game/BP/BP_NotePool.GetNote` (`self.NotePool`)))
        (bind _spawnpos (`self.ConvertOsuPosToSpawnPos` _osux _osuy))
        (`/Game/BP/BP_Note.Setup` _note _hittime (`KismetMathLibrary.MakeVector` (`KismetMathLibrary.BreakVector2D` _spawnpos) (`.Y` (`KismetMathLibrary.BreakVector2D` _spawnpos)) _returnvalue_2) (`KismetMathLibrary.MakeVector` _returnvalue_x _returnvalue_y _returnvalue_2) (`self.MusicManager`) self (`self.TravelTime`) _hitsound)
        (`KismetArrayLibrary.Array_Add` (`/Game/BP/BP_HitJudgementManager.NoteQueue` (`self.HitJudgementManager`)) _note)
        (`/Engine/EditorBlueprintResources/StandardMacros.IncrementInt` (`self.CurrentNoteIndex`))
        (else
          (break))))))

(fn `ConvertOsuPosToSpawnPos`
  (params (OsuX :type Integer) (OsuY :type Integer))
  (returns (SpawnPos :type "Vector2D Structure"))
  (bind _spawndistance (`self.SpawnDistance`))
  (bind (_returnvalue_x _returnvalue_y) (`KismetMathLibrary.BreakVector2D` (`KismetMathLibrary.Normal2D` (- (`KismetMathLibrary.MakeVector2D` (`KismetMathLibrary.Conv_IntToDouble` OsuX) (`KismetMathLibrary.Conv_IntToDouble` OsuY)) (256.0 256.0)))))
  (return (`KismetMathLibrary.MakeVector2D` (* _returnvalue_x _spawndistance) (* _returnvalue_y _spawndistance))))

(fn `InitNoteArray`
  (bind _beatmaparray (`self.BeatmapArray`))
  (bind _outrownames (`DataTableFunctionLibrary.GetDataTableRowNames` "/Game/testmap.testmap"))
  (`KismetArrayLibrary.Array_Clear` _beatmaparray)
  (for _array_element _outrownames
    (bind _returnvalue (`|GetDataTableRow` "/Game/testmap.testmap" _array_element)
      (:`then`
        (`KismetArrayLibrary.Array_Add` _beatmaparray _returnvalue)))))

(fn `NoteSpawnDebug`
  (params (noteObject :type "/Game/BP/BP_Note Object Reference") (hitTime :type Integer) (startPos :type "Vector Structure") (targetPos :type "Vector Structure"))
  (`KismetSystemLibrary.PrintString` (`KismetStringLibrary.Concat_StrStr` (`KismetStringLibrary.Concat_StrStr` (`KismetStringLibrary.Concat_StrStr` (`KismetStringLibrary.Concat_StrStr` (`KismetStringLibrary.Concat_StrStr` (`KismetStringLibrary.Concat_StrStr` (`KismetSystemLibrary.GetObjectName` noteObject) " hitTime: ") (`KismetStringLibrary.Conv_IntToString` hitTime)) " StartPos: ") (`KismetStringLibrary.Conv_VectorToString` startPos)) " TargetPos: ") (`KismetStringLibrary.Conv_VectorToString` targetPos))))

(fn `PauseMap`
  (bind _musicmanager (`self.MusicManager`))
  (bind _pausemenuobj (`self.PauseMenuObj`))
  (`self.isMapRunning`
    (:`then`
      (bind _output_get (set `self.isPaused` (not (`self.isPaused`))))
      (if _output_get
        ; UI
        (`/Engine/EditorBlueprintResources/StandardMacros.IsValid` _pausemenuobj
          (:`Is Valid`
            (`Widget.SetVisibility` _pausemenuobj "Visible"))
          (:`Is Not Valid`
            (bind _returnvalue (`|CreateWidget` "/Game/BP/WBP_PauseMenu.WBP_PauseMenu_C"))
            (set `/Game/BP/WBP_PauseMenu.GameFlow` self _returnvalue)
            (set `self.PauseMenuObj` _returnvalue)
            (`UserWidget.AddToViewport` _returnvalue 0)))
        (`/Game/BP/BP_MusicManager.SetPaused` _musicmanager true)
        (else
          (`/Engine/EditorBlueprintResources/StandardMacros.IsValid` _pausemenuobj
            (:`Is Valid`
              (`Widget.SetVisibility` _pausemenuobj "Hidden")
              (`/Game/BP/BP_MusicManager.SetPaused` _musicmanager false))))))
    (:`else`)))

(fn `RestartMap`
  (bind _pausemenuobj (`self.PauseMenuObj`))
  (bind _notequeue (`/Game/BP/BP_HitJudgementManager.NoteQueue` (`self.HitJudgementManager`)))
  ; UI
  (`/Engine/EditorBlueprintResources/StandardMacros.IsValid` _pausemenuobj
    (:`Is Valid`
      (`Widget.SetVisibility` _pausemenuobj "Hidden"))
    (:`Is Not Valid`
      _))
  (for _array_element _notequeue
    (`/Game/BP/BP_NotePool.ReturnNote` (`self.NotePool`) _array_element))
  (`KismetArrayLibrary.Array_Clear` _notequeue)
  (set `self.CurrentNoteIndex` 0)
  (set `self.isPaused` false)
  (`/Game/BP/BP_MusicManager.StopMusic` (`self.MusicManager`))
  (`self.StartGame`))

(fn `SolveOnNoteHit`
  (params (Note :type "/Game/BP/BP_Note Object Reference"))
  (`KismetArrayLibrary.Array_RemoveItem` (`/Game/BP/BP_HitJudgementManager.NoteQueue` (`self.HitJudgementManager`)) Note)
  (`/Game/BP/BP_NotePool.ReturnNote` (`self.NotePool`) Note))

(fn `StartGame`
  (bind _musicmanager (`self.MusicManager`))
  (bind _beatmaparray (`self.BeatmapArray`))
  (bind (_output_osux _output_osuy _output_hittime) (break `/Game/BP/STR_NoteInfo` (`|GetArrayItem` _beatmaparray)))
  (if (!= (`KismetArrayLibrary.Array_Length` _beatmaparray) 0)
    (if (< _output_hittime 1000)
      (`/Game/BP/BP_MusicManager.SetCurrentTime` _musicmanager (* (`self.TravelTime`) -1.0))
      (else
        (`/Game/BP/BP_MusicManager.SetPaused` _musicmanager false)
        (`/Game/BP/BP_MusicManager.PlayMusic` _musicmanager "/Game/Audio/Rick_Astley_-_Never_Gonna_Give_You_Up__Besai_Remix_.Rick_Astley_-_Never_Gonna_Give_You_Up__Besai_Remix_")))
    (set `self.isMapRunning` true)))

(fn `UserConstructionScript`)