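; BP_HitEffectManager spawns animated hit effects when notes are hit, in what appears to be a rhythm game.
; On BeginPlay it binds to HitJudgementManager's OnNoteHit event.
; Each hit takes an effect from an ObjectPool and plays its animation for the judgement result, printing a debug string if none is valid.
; When the animation ends, the effect unbinds its listeners and returns to the pool.
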(event `OnHitEffectAnimEnd`
  (params (HitEffectSelf :type "/Game/BP/BP_HitEffect Object Reference"))
  (clear `/Game/BP/BP_HitEffect.OnAnimEnd` HitEffectSelf)
  (`/Game/BP/BP_HitEffectPool.ReturnObj` (`self.ObjectPool`) HitEffectSelf))

(event `OnNoteHit`
  (params (Note :type "/Game/BP/BP_Note Object Reference") (Result :type "/Game/BP/NoteHitResult Enum" :default "NewEnumerator0"))
  (bind _obj (`/Game/BP/BP_HitEffectPool.GetObj` (`self.ObjectPool`)))
  (`/Engine/EditorBlueprintResources/StandardMacros.IsValid` _obj
    (:`Is Valid`
      (add `/Game/BP/BP_HitEffect.OnAnimEnd` _obj (delegate `OnHitEffectAnimEnd`))
      (`/Game/BP/BP_HitEffect.PlayAnim` _obj Result))
    (:`Is Not Valid`
      (`KismetSystemLibrary.PrintString` "NOT VALID MY ASS"))))

(event `self.ReceiveBeginPlay`
  (add `/Game/BP/BP_HitJudgementManager.OnNoteHit` (`self.HitJudgementManager`) (delegate `OnNoteHit`)))

(fn `UserConstructionScript`)