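; BP_MusicPlayer is a music player actor that tracks the current song time on a Quartz clock it creates at BeginPlay.
; UpdateCurrentTime feeds the clock's timestamp through SolveQuartzPlayTimeStamp and returns CurrentTime.
; While CurrentTime is negative, nonzero readings are flagged as leftovers from the previous track, and their timestamp gates later updates to filter stale values.
; A duplicate solver based on audio playback percent remains, but its event binding is disconnected.
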(event `self.ReceiveBeginPlay`
  (add `self.OnDestroyed` (delegate `OnDestroyed_Event`))
  (bind _returnvalue (`QuartzSubsystem.CreateNewClock` :`self` (subsystem `QuartzSubsystem`) :`ClockName` "Main"))
  (set `self.QuartzClockHandle` _returnvalue))

(event `OnAudioPlaybackPercent_Event`
  (params (PlayingSoundWave :type "SoundWave Object Reference") (PlaybackPercent :type "Float (single-precision)"))
  ; set current time on music play
  (`self.SolveAudioPlaybackPercent` PlayingSoundWave PlaybackPercent))

(event `self.ReceiveTick`
  (params (DeltaSeconds :type "Float (single-precision)")))

(event `OnDestroyed_Event` :!signature `self.OnDestroyed`
  (params (DestroyedActor :type "Actor Object Reference"))
  (remove `AudioComponent.OnAudioPlaybackPercent` (`self.Audio`) (delegate `OnAudioPlaybackPercent_Event`))
  (remove `self.OnDestroyed` (delegate `OnDestroyed_Event`)))

(fn `SolveAudioPlaybackPercent`
  (params (Sound :type "SoundWave Object Reference") (PlaybackPercent :type "Float (double-precision)"))
  (bind _pausetimestamp (`self.PauseTimeStamp`))
  (bind _returnvalue (* PlaybackPercent (`SoundBase.Duration` Sound)))
  (if (< (`self.CurrentTime`) 0.0)
    (if (!= _returnvalue 0.0)
      (set `self.HaveUncleanedTrack` true)
      (set `self.PauseTimeStamp` _returnvalue))
    (else
      (`self.HaveUncleanedTrack`
        (:`then`
          (if (< (- _pausetimestamp (`self.CurrentTime`)) 0.5)
            (set `self.HaveUncleanedTrack` false)
            (set `self.CurrentTime` _returnvalue :!label _label)
            (elif (< _returnvalue _pausetimestamp)
              (goto _label))))
        (:`else`
          (goto _label))))))

(fn `SolveQuartzPlayTimeStamp`
  (params (Seconds :type "Float (double-precision)"))
  (bind _pausetimestamp (`self.PauseTimeStamp`))
  ; If curr is negative but music api sends value that is not 0, that means we have previous song track value to deal with
  (if (< (`self.CurrentTime`) 0.0)
    (if (!= Seconds 0.0)
      (set `self.HaveUncleanedTrack` true)
      (set `self.PauseTimeStamp` Seconds))
    (else
      (`self.HaveUncleanedTrack`
        (:`then`
          (if (< (- _pausetimestamp (`self.CurrentTime`)) 0.5)
            (set `self.HaveUncleanedTrack` false)
            (set `self.CurrentTime` Seconds :!label _label)
            (elif (< Seconds _pausetimestamp)
              (goto _label))))
        (:`else`
          (goto _label))))))

(fn `UpdateCurrentTime`
  (returns (CurrentTime :type "Float (double-precision)"))
  (bind _returnvalue (`QuartzClockHandle.GetCurrentTimestamp` (`self.QuartzClockHandle`)))
  (`self.SolveQuartzPlayTimeStamp` (`.Seconds` (break `QuartzTransportTimeStamp` _returnvalue)))
  (return (`self.CurrentTime`)))

(fn `UserConstructionScript`)