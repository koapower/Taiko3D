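; Hit judgement manager for a Taiko-style rhythm game, grading Don and Ka drum inputs against queued notes.
; On BeginPlay it derives Great, Ok and Miss windows from the OD setting and binds to player controller drum events.
; Each input plays its sound, clears overdue notes as misses, then tests the front note against widening windows using music time.
; Results go out through OnNoteHit, with wrong-color hits counting as misses.
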(event `OnDon`
  (params (DrumInput :type "/Game/Input/DrumInputType Enum" :default "NewEnumerator0"))
  (`/Game/BP/BP_MusicManager.PlaySound2D` (`self.MusicManager`) "/Game/Audio/MSS_DON.MSS_DON")
  (`self.HandleInputEvent` DrumInput))

(event `self.ReceiveBeginPlay`
  (`self.Init`)
  (bind _asbp_taiko_player_controller (cast `/Game/BP_TaikoPlayerController` (`GameplayStatics.GetPlayerController` 0)))
  (add `/Game/BP_TaikoPlayerController.OnDon` _asbp_taiko_player_controller (delegate `OnDon`))
  (add `/Game/BP_TaikoPlayerController.OnKa` _asbp_taiko_player_controller (delegate `OnKa`)))

(event `OnKa`
  (params (DrumInput :type "/Game/Input/DrumInputType Enum" :default "NewEnumerator0"))
  (`/Game/BP/BP_MusicManager.PlaySound2D` (`self.MusicManager`) "/Game/Audio/MSS_KA.MSS_KA")
  (`self.HandleInputEvent` DrumInput))

(fn `ClearMissedNotes`
  (locals (MissResult :type "/Game/BP/NoteHitResult Enum"))
  (bind _temparray (`self.tempArray`))
  (for _array_element (`self.NoteQueue`)
    (bind _diffms (`self.GetHitTimeDiffMs` _array_element))
    (bind _returnvalue (< _diffms (* (`self.MissMs`) -1)))
    (if _returnvalue
      (`KismetArrayLibrary.Array_Add` _temparray _array_element)
      (`KismetSystemLibrary.PrintText` (`|FormatText` "ClearMiss: {0} hitTime: {2} diff: {1} needDelete: {3}" _array_element _diffms (`/Game/BP/BP_Note.HitTime_ms` _array_element) _returnvalue))
      (else
        (break))))
  (for _array_element_2 _temparray
    (`self.OnNoteHit` _array_element_2 "NewEnumerator0")
    (`KismetSystemLibrary.PrintString` "clearmissednotes"))
  (`KismetArrayLibrary.Array_Clear` _temparray))

(fn `ConvertDrumInputToNoteType`
  (params (DrumInput :type "/Game/Input/DrumInputType Enum" :default "NewEnumerator0"))
  (returns (NoteType :type Integer))
  (locals (NewLocalVar :type Integer))
  (switch `/Game/Input/DrumInputType` DrumInput
    (:`NewEnumerator0`
      _)
    (:`NewEnumerator1`
      _)
    (:`NewEnumerator2`
      (bind _output_get (set `local.NewLocalVar` 8 :!label _label))
      (return _output_get))
    (:`NewEnumerator3`
      (goto _label)))
  (bind _output_get_2 (set `local.NewLocalVar` 0))
  (return _output_get_2))

(fn `GetHitTimeDiffMs`
  (params (Note :type "/Game/BP/BP_Note Object Reference"))
  (returns (diffMs :type Integer))
  (return (- (`/Game/BP/BP_Note.HitTime_ms` Note) (* (`/Game/BP/BP_MusicManager.CurrentTime` (`self.MusicManager`)) 1000.0))))

(fn `HandleInputEvent`
  (params (DrumInput :type "/Game/Input/DrumInputType Enum" :default "NewEnumerator0"))
  (locals (Result :type "/Game/BP/NoteHitResult Enum"))
  (bind _notequeue (`self.NoteQueue`))
  (bind _output (`|GetArrayItem` _notequeue))
  (bind _returnvalue (!= (`KismetArrayLibrary.Array_Length` _notequeue) 0))
  (if (and (`self._inited`) _returnvalue)
    (`self.ClearMissedNotes`)
    (if _returnvalue
      (bind _diffms (`self.GetHitTimeDiffMs` _output))
      (bind _notetype (`self.ConvertDrumInputToNoteType` DrumInput))
      (bind _returnvalue_2 (`KismetMathLibrary.Abs_Int` _diffms))
      (bind _issuccess (`self.JudgeTiming` _returnvalue_2 (`self.GreatMs`) _notetype _output "NewEnumerator2"))
      (if (not _issuccess)
        (bind _issuccess_2 (`self.JudgeTiming` _returnvalue_2 (`self.OkMs`) _notetype _output "NewEnumerator1"))
        (if (not _issuccess_2)
          (`self.JudgeTiming` _returnvalue_2 (`self.MissMs`) _notetype _output))))))

(fn `Init`
  (bind (_settings_od _settings_greatfixedms _settings_okfixedms_lowod _settings_okfixedms_highod _settings_missfixedms_lowod _settings_missfixedms_highod _settings_greatodmultiplier _settings_okodmultiplier_lowod _settings_okodmultiplier_highod _settings_missodmultiplier_lowod _settings_missodmultiplier_highod) (break `/Game/BP/STR_HitJudgingSettings` (`self.Settings`)))
  (set `self.GreatMs` (- _settings_greatfixedms (* _settings_od _settings_greatodmultiplier)))
  (if (< _settings_od 5.0)
    ; LowerOD
    (set `self.OkMs` (- _settings_okfixedms_lowod (* _settings_od _settings_okodmultiplier_lowod)))
    (set `self.MissMs` (- _settings_missfixedms_lowod (* _settings_od _settings_missodmultiplier_lowod)))
    (else
      ; HigherOD
      (set `self.OkMs` (- _settings_okfixedms_highod (* _settings_od _settings_okodmultiplier_highod)))
      (set `self.MissMs` (- _settings_missfixedms_highod (* _settings_od _settings_missodmultiplier_highod)))))
  (set `self._inited` true))

(fn `InputIsCorrectType`
  (params (Type :type Integer) (Note :type "/Game/BP/BP_Note Object Reference"))
  (returns (isCorrect :type Boolean))
  (return (== Type (`/Game/BP/BP_Note.NoteType` Note))))

(fn `JudgeTiming`
  (params (AbsDiffMs :type Integer) (HitWindowMs :type Integer) (InputType :type Integer) (Note :type "/Game/BP/BP_Note Object Reference") (ResultIfSuccess :type "/Game/BP/NoteHitResult Enum" :default "NewEnumerator0"))
  (returns (IsSuccess :type Boolean))
  (locals (Result :type "/Game/BP/NoteHitResult Enum"))
  (if (<= AbsDiffMs HitWindowMs)
    (bind _iscorrect (`self.InputIsCorrectType` InputType Note))
    (if _iscorrect
      (set `local.Result` ResultIfSuccess)
      (else
        (set `local.Result` "NewEnumerator0")))
    (`self.OnNoteHit` Note (`local.Result`))
    (return true)
    (else
      (return false))))

(fn `UserConstructionScript`)