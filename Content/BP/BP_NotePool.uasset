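; BP_NotePool is an object pool that supplies reusable BP_Note actors.
; BeginPlay pre-spawns notes through SpawnNote, hidden and with tick disabled, into InPoolNotes.
; GetNote moves the first pooled note to ActiveNotes, or spawns one when empty, though that new note also stays in InPoolNotes.
; ReturnNote resets a note and moves it back to the pool.
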(event `self.ReceiveBeginPlay`
  (for _ (range (+ (`self.PoolSize`) 1))
    (`self.SpawnNote`)))

(fn `GetNote`
  (returns (Note :type "/Game/BP/BP_Note Object Reference"))
  (locals (NoteFromPool :type "/Game/BP/BP_Note Object Reference"))
  (bind _inpoolnotes (`self.InPoolNotes`))
  (bind _activenotes (`self.ActiveNotes`))
  (if (== (`KismetArrayLibrary.Array_Length` (`self.InPoolNotes`)) 0)
    (bind _note (`self.SpawnNote`))
    (`KismetArrayLibrary.Array_Add` _activenotes _note)
    (return _note)
    (else
      (bind _output_get (set `local.NoteFromPool` (`|GetArrayItem` _inpoolnotes)))
      (`KismetArrayLibrary.Array_Remove` _inpoolnotes)
      (`KismetArrayLibrary.Array_Add` _activenotes _output_get)
      (return _output_get))))

(fn `ReturnNote`
  (params (Note :type "/Game/BP/BP_Note Object Reference"))
  (`/Game/BP/BP_Note.Reset` Note)
  (`KismetArrayLibrary.Array_RemoveItem` (`self.ActiveNotes`) Note)
  (`KismetArrayLibrary.Array_Add` (`self.InPoolNotes`) Note))

(fn `SpawnNote`
  (returns (Note :type "/Game/BP/BP_Note Object Reference"))
  (locals (NewLocalVar :type "/Game/BP/BP_Note Object Reference"))
  (bind _returnvalue (`|SpawnActorFromClass` "/Game/BP/BP_Note.BP_Note_C" (`KismetMathLibrary.Conv_VectorToTransform` (0.0 0.0 0.0)) "Undefined" "MultiplyWithRoot" null null))
  (`self.SetActorHiddenInGame` _returnvalue true)
  (`self.SetActorTickEnabled` _returnvalue false)
  (`KismetArrayLibrary.Array_Add` (`self.InPoolNotes`) _returnvalue)
  (return _returnvalue))

(fn `UserConstructionScript`)