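; BP_ScoreSystem is an actor that tracks the player's current combo from note hit results.
; On BeginPlay it binds to HitJudgementManager's OnNoteHit event and passes each result to SolveOnNoteHit.
; That function resets the combo on the enum's NewEnumerator0 result and increments it on any other.
; ResetScore only zeroes the combo, as no score value is tracked here.
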(event `OnNoteHit`
  (params (Note :type "/Game/BP/BP_Note Object Reference") (Result :type "/Game/BP/NoteHitResult Enum" :default "NewEnumerator0"))
  (`self.SolveOnNoteHit` Note Result))

(event `self.ReceiveBeginPlay`
  (add `/Game/BP/BP_HitJudgementManager.OnNoteHit` (`self.HitJudgementManager`) (delegate `OnNoteHit`)))

(fn `ResetScore`
  (set `self.CurrentCombo` 0))

(fn `SolveOnNoteHit`
  (params (Note :type "/Game/BP/BP_Note Object Reference") (HitResult :type "/Game/BP/NoteHitResult Enum" :default "NewEnumerator0"))
  (locals (ResultMiss :type "/Game/BP/NoteHitResult Enum"))
  (if (`|EnumInequality` HitResult "NewEnumerator0")
    (`/Engine/EditorBlueprintResources/StandardMacros.IncrementInt` (`self.CurrentCombo`))
    (else
      (set `self.CurrentCombo` 0))))

(fn `UserConstructionScript`)