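; BP_HitEffectPool is an object pool that reuses BP_HitEffect actors.
; BeginPlay pre-spawns a batch at the origin, hidden with tick disabled, into InPoolArr.
; GetObj and ReturnObj move actors between InPoolArr and ActiveArr without changing visibility or tick.
; When the pool is empty, GetObj spawns a new actor, which lands in both arrays because SpawnObj also adds it to InPoolArr.
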(event `self.ReceiveBeginPlay`
  (for _ (range 31)
    (`self.SpawnObj`)))

(fn `GetObj`
  (returns (Obj :type "/Game/BP/BP_HitEffect Object Reference"))
  (locals (ObjFromPool :type "/Game/BP/BP_HitEffect Object Reference"))
  (bind _inpoolarr (`self.InPoolArr`))
  (bind _activearr (`self.ActiveArr`))
  (if (== (`KismetArrayLibrary.Array_Length` (`self.InPoolArr`)) 0)
    (bind _obj (`self.SpawnObj`))
    (`KismetArrayLibrary.Array_Add` _activearr _obj)
    (return _obj)
    (else
      (bind _output_get (set `local.ObjFromPool` (`|GetArrayItem` _inpoolarr)))
      (`KismetArrayLibrary.Array_Remove` _inpoolarr)
      (`KismetArrayLibrary.Array_Add` _activearr _output_get)
      (return _output_get))))

(fn `ReturnObj`
  (params (Obj :type "/Game/BP/BP_HitEffect Object Reference"))
  (`KismetArrayLibrary.Array_RemoveItem` (`self.ActiveArr`) Obj)
  (`KismetArrayLibrary.Array_Add` (`self.InPoolArr`) Obj))

(fn `SpawnObj`
  (returns (Obj :type "/Game/BP/BP_HitEffect Object Reference"))
  (locals (NewLocalVar :type "/Game/BP/BP_Note Object Reference"))
  (bind _returnvalue (`|SpawnActorFromClass` "/Game/BP/BP_HitEffect.BP_HitEffect_C" (`KismetMathLibrary.Conv_VectorToTransform` (0.0 0.0 0.0)) "Undefined" "MultiplyWithRoot" null null))
  (`self.SetActorHiddenInGame` _returnvalue true)
  (`self.SetActorTickEnabled` _returnvalue false)
  (`KismetArrayLibrary.Array_Add` (`self.InPoolArr`) _returnvalue)
  (return _returnvalue))

(fn `UserConstructionScript`)